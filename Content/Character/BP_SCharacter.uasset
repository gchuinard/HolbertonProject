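; Player character Blueprint that adds a health indicator widget at BeginPlay when locally controlled and uses M to toggle a menu widget, cursor and pause.
; CheckifEnemy line-traces from the camera, intended for crosshair coloring, and re-calls itself after a short delay only when nothing is hit.
; Its Friendly, Neutral and Enemy flag logic is disconnected, and nothing else in this graph starts the check.
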(event `Check if Enemy`
  (bind _cameracomp (`self.CameraComp`))
  (bind _returnvalue (`SceneComponent.K2_GetComponentLocation` _cameracomp))
  ;[1 1 1] Crosshair color
  (bind (_outhit _returnvalue_2) (`KismetSystemLibrary.LineTraceSingle` _returnvalue (+ _returnvalue (* (`SceneComponent.GetForwardVector` _cameracomp) 10000.0)) "TraceTypeQuery1"))
  (if _returnvalue_2
    (if (`self.ActorHasTag` (`.HitActor` (`GameplayStatics.BreakHitResult` _outhit)) "Ally")
      _)
    (else
      (`KismetSystemLibrary.Delay` 0.01)
      (`self.Check if Enemy`))))

(event `Key|M` :paused true
  (params (Key :type "Key Structure"))
  (bind _returnvalue (`GameplayStatics.GetPlayerController` 0))
  (:`Pressed`
    (`/Engine/EditorBlueprintResources/StandardMacros.FlipFlop`
      (:`A`
        (bind _returnvalue_2 (`|CreateWidget` "/Game/UI/NewWidgetBlueprint.NewWidgetBlueprint_C"))
        (`UserWidget.AddToViewport` _returnvalue_2 0)
        (set `PlayerController.bShowMouseCursor` true _returnvalue)
        (`GameplayStatics.SetGamePaused` true))
      (:`B`
        (`Widget.RemoveFromParent` _returnvalue_2)
        (set `PlayerController.bShowMouseCursor` false _returnvalue)
        (`GameplayStatics.SetGamePaused` false)))))

(event `self.ReceiveBeginPlay`
  (if (`self.IsLocallyControlled`)
    (bind _returnvalue (`|CreateWidget` "/Game/UI/WBP_HealthIndicator.WBP_HealthIndicator_C"))
    (`/Engine/EditorBlueprintResources/StandardMacros.IsValid` _returnvalue
      (:`Is Valid`
        (`UserWidget.AddToViewport` _returnvalue 0)))))

(fn `UserConstructionScript`)