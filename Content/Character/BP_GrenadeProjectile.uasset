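; Grenade projectile actor that explodes on a timed fuse after it spawns.
; BeginPlay waits for Duration, then Explode spawns an emitter and sound, applies radial damage credited to the instigator's controller, and destroys the actor.
; An H key handler prints and cycles this instance's Duration in one-second steps, wrapping at the upper limit.
; The fuse reads Duration when BeginPlay starts the delay, so later changes leave the running countdown unchanged.
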(event `self.ReceiveBeginPlay`
  (`KismetSystemLibrary.Delay` (`self.Duration`))
  (`self.Explode`))

(event `Key|H`
  (params (Key :type "Key Structure"))
  (bind _duration (`self.Duration`))
  (bind _duration_2 (`self.Duration`))
  (:`Pressed`
    (`KismetSystemLibrary.PrintString` "Hello")
    (if (< _duration 5.0)
      (`KismetSystemLibrary.PrintString` (`KismetStringLibrary.Conv_DoubleToString` _duration_2))
      (set `self.Duration` (+ _duration 1.0))
      (else
        (`KismetSystemLibrary.PrintString` (`KismetStringLibrary.Conv_DoubleToString` _duration_2))
        (set `self.Duration` 1.0)))))

(event `Explode`
  (bind _returnvalue (`self.K2_GetActorLocation`))
  (`GameplayStatics.SpawnEmitterAtLocation` "/Game/M5_Vol1/Particles/Normal_Explosion/N_RealExp_00_C.N_RealExp_00_C" _returnvalue)
  (`GameplayStatics.SpawnSoundAtLocation` "/Game/Gun_Explosion_Sounds/Explosions/wav/Thick_Explosion_01.Thick_Explosion_01" _returnvalue (struct) 1.0 1.0 0.0 null null)
  (`GameplayStatics.ApplyRadialDamage` :`BaseDamage` 75.0 :`Origin` _returnvalue :`DamageRadius` (`self.Damage Radius`) :`DamageCauser` self :`InstigatedByController` (`self.GetInstigatorController`))
  (`self.K2_DestroyActor`))

(fn `UserConstructionScript`)