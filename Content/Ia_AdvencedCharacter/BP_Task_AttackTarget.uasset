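; Behavior tree task that makes an AI-controlled SCharacter fire a burst of shots when attacking.
; On execute it picks a random branch, each a hard-coded chain of FtPullTrigger calls spaced by short Delays, so burst length varies.
; After the burst it finishes execution as failed, while a failed SCharacter cast calls FinishAbort.
; A longer trigger chain and an empty ElseIf graph are unused.
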(event `self.ReceiveExecuteAI`
  (params (OwnerController :type "AIController Object Reference") (ControlledPawn :type "Pawn Object Reference"))
  (bind _asscharacter (cast `SCharacter` ControlledPawn)
    (:`then`
      (switch `int` (`KismetMathLibrary.RandomIntegerInRange` 0 5)
        (:`Default`
          (`KismetSystemLibrary.Delay` 0.2 :!label _label)
          (`SCharacter.FtPullTrigger` _asscharacter)
          (`KismetSystemLibrary.Delay` 0.2)
          (`SCharacter.FtPullTrigger` _asscharacter)
          (`KismetSystemLibrary.Delay` 0.2)
          (`SCharacter.FtPullTrigger` _asscharacter)
          (`KismetSystemLibrary.Delay` 0.2)
          (`SCharacter.FtPullTrigger` _asscharacter))
        (:`0`
          (goto _label))
        (:`1`
          (`KismetSystemLibrary.Delay` 0.2)
          (`SCharacter.FtPullTrigger` _asscharacter)
          (`KismetSystemLibrary.Delay` 0.2)
          (`SCharacter.FtPullTrigger` _asscharacter))
        (:`2`
          (`KismetSystemLibrary.Delay` 0.2)
          (`SCharacter.FtPullTrigger` _asscharacter)
          (`KismetSystemLibrary.Delay` 0.2)
          (`SCharacter.FtPullTrigger` _asscharacter)
          (`KismetSystemLibrary.Delay` 0.2)
          (`SCharacter.FtPullTrigger` _asscharacter)
          (`KismetSystemLibrary.Delay` 0.2)
          (`SCharacter.FtPullTrigger` _asscharacter)
          (`KismetSystemLibrary.Delay` 0.2)
          (`SCharacter.FtPullTrigger` _asscharacter)
          (`KismetSystemLibrary.Delay` 0.2)
          (`SCharacter.FtPullTrigger` _asscharacter))
        (:`3`
          (`SCharacter.FtPullTrigger` _asscharacter)
          (`KismetSystemLibrary.Delay` 0.2)
          (`SCharacter.FtPullTrigger` _asscharacter)
          (`KismetSystemLibrary.Delay` 0.2)
          (`SCharacter.FtPullTrigger` _asscharacter))
        (:`4`
          (`KismetSystemLibrary.Delay` 0.2)
          (`SCharacter.FtPullTrigger` _asscharacter)
          (`KismetSystemLibrary.Delay` 0.2)
          (`SCharacter.FtPullTrigger` _asscharacter)
          (`KismetSystemLibrary.Delay` 0.2)
          (`SCharacter.FtPullTrigger` _asscharacter)
          (`KismetSystemLibrary.Delay` 0.2)
          (`SCharacter.FtPullTrigger` _asscharacter)
          (`KismetSystemLibrary.Delay` 0.2)
          (`SCharacter.FtPullTrigger` _asscharacter)))
      (`self.FinishExecute` false))
    (:`CastFailed`
      (`self.FinishAbort`))))